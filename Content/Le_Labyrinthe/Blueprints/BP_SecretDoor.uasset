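; BP_SecretDoor is the labyrinth's secret door, which opens only when both a lever and a torch puzzle condition are met.
; Its OpenDoor event finds one BP_Levier and one BP_Torche by class and checks that the lever is unlocked and the torch lit.
; On success it destroys its owner (GetOwner, not Self); otherwise it prints a message that conditions are not met.
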(event Custom|OpenDoor
  ;[1 1 1] Checks if the lever and the torch are activated
  (bind _returnvalue (Actor|GetActorOfClass "/Game/Le_Labyrinthe/Blueprints/BP_Levier.BP_Levier_C"))
  (bind _asbp_levier (Utilities|Casting|CastToBP_Levier _returnvalue))
  (bind _returnvalue_2 (Actor|GetActorOfClass "/Game/Le_Labyrinthe/Blueprints/BP_Torche.BP_Torche_C"))
  (bind _asbp_torche (Utilities|Casting|CastToBP_Torche _returnvalue_2))
  (if (and (Variables|/Game/Le_Labyrinthe/Blueprints/BP_Levier.BP_Levier_C|GetUnlocked _asbp_levier) (Variables|/Game/Le_Labyrinthe/Blueprints/BP_Torche.BP_Torche_C|GetLit _asbp_torche))
    (Actor|DestroyActor (Components|GetOwner self))
    (else
      (Development|PrintString "Not all conditions met !" true true "(R=1.000000,G=0.000000,B=0.029223,A=1.000000)"))))

(event EventBeginPlay)