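; BP_Piège is a spike trap actor for the labyrinth (Le_Labyrinthe) that reveals itself when something overlaps it.
; On BeginPlay it hides its text render and six spike components.
; ActorBeginOverlap makes them visible again, with no filter on the overlapping actor, no damage logic and no re-hide.
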(event EventBeginPlay
  (Rendering|SetVisibility (Variables|Default|GetTextRender) false false)
  (Rendering|SetVisibility (Variables|Default|Getspike1) false false))

(event Collision|EventActorBeginOverlap
  (params (OtherActor :type Actor%20Object%20Reference))
  (Rendering|SetVisibility (Variables|Default|GetTextRender) true false)
  (Rendering|SetVisibility (Variables|Default|Getspike1) true false))

(event EventTick
  (params (DeltaSeconds :type Float%20%28single-precision%29)))

(fn ConstructionScript)