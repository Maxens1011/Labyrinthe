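; BP_Levier is a lever that opens secret doors when activated.
; ActivateLever sets an Unlocked flag, then scans every StaticMeshActor in the level and calls OpenDoor on its BP_SecretDoor component, without a validity check.
; The same loop reveals the activation text, which BeginPlay hides, and the Cone mesh then snaps to a fixed world rotation.
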(event Custom|ActivateLever
  ;[1 1 1] Unlocks Door
  (Variables|Default|SetUnlocked true)
  (bind _outactors (Actor|GetAllActorsOfClass "/Script/Engine.StaticMeshActor"))
  (for _array_element _outactors
    (Default|OpenDoor (Actor|GetComponentbyClass _array_element "/Game/Le_Labyrinthe/Blueprints/BP_SecretDoor.BP_SecretDoor_C"))
    ;[1 1 1] Turns text on
    (Rendering|SetVisibility (Variables|Default|GetActivation%20text) true false))
  (Transformation|SetWorldRotation (Variables|Default|GetCone) "180.000000,0.000000,0.000000" false false))

(event EventBeginPlay
  ;[1 1 1] Turns text  on at start
  (Rendering|SetVisibility (Variables|Default|GetActivation%20text) false false))

(fn ConstructionScript)